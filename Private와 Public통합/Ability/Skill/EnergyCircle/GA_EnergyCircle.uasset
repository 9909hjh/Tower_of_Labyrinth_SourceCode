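; GA_EnergyCircle is a Gameplay Ability for the katana character's Energy Circle skill, playing one attack montage per activation.
; After committing cost and cooldown, it calls DirectionCameraLookingAt on the character and plays the montage indexed by CurrentAttackCount, cancelling if commit or cast fails.
; The counter advances cyclically through five montages, and the ability ends when the montage finishes or is interrupted.
; AttackAnimCheak and HitAnimCheak contain only unconnected nodes.
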(event Ability|EventActivateAbility
  (bind _montage_to_play_attack_1 (Variables|공격콤보|GetMontage%20to%20Play_Attack_1))
  (bind _montage_to_play_attack_2 (Variables|공격콤보|GetMontage%20to%20Play_Attack_2))
  (bind _montage_to_play_attack_3 (Variables|공격콤보|GetMontage%20to%20Play_Attack_3))
  (bind _montage_to_play_attack_4 (Variables|공격콤보|GetMontage%20to%20Play_Attack_4))
  (bind _montage_to_play_attack_0 (Variables|공격콤보|GetMontage%20to%20Play_Attack_0))
  (bind _array (Utilities|Array|MakeArray _montage_to_play_attack_0 _montage_to_play_attack_1 _montage_to_play_attack_2 _montage_to_play_attack_3 _montage_to_play_attack_4))
  (bind _returnvalue (Utilities|Array|Length _array))
  (bind _returnvalue_2 (Ability|CommitAbility))
  (if _returnvalue_2 ; 쿨타임이 돌았거나 비용이 있다면!
    (bind _asbp_katana_character_base (Utilities|Casting|CastToBP_KatanaCharacterBase (Ability|GetAvatarActorfromActorInfo))
      (:then
        (bind _output_get (Variables|Default|SetAs%20BP%20Katana%20Character%20Base _asbp_katana_character_base))
        (Class|KatanaCharacterBase|DirectionCameraLookingat _output_get)
        (Variables|공격콤보|SetAttackMontageArrayLength _returnvalue)
        (if (not (<= _returnvalue 0))
          (|PlayMontageandWaitProxy "None" (Utilities|Array|Get(acopy) _array (Variables|공격콤보|GetCurrentAttackCount)) 1.0 "None" true 1.0 0.0
            (:then
              (if (>= (+ (Variables|공격콤보|GetCurrentAttackCount) 1) (Variables|공격콤보|GetAttackMontageArrayLength))
                (Variables|공격콤보|SetCurrentAttackCount 0)
                (else
                  (bind _result (Math|Integer|IncrementInt (Variables|공격콤보|GetCurrentAttackCount))
                    (:%20%20
                      (Variables|공격콤보|SetCurrentAttackCount _result))))))
            (:OnCompleted
              (Ability|EndAbility :!label _label))
            (:OnBlendOut
              (goto _label))
            (:OnInterrupted
              (goto _label))
            (:OnCancelled
              (goto _label)))))
      (:CastFailed
        (Ability|CancelAbility :!label _label_2) ; 쿨타임 중이거나 비용이 없다면 어빌리티 취소
      ))
    (else
      (goto _label_2))))