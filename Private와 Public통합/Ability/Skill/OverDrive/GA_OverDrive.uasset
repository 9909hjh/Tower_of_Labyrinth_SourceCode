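; GA_OverDrive is the katana character's Overdrive gameplay ability, trading 30% of max health for a timed strength and attack-speed buff.
; Activation cancels during a dash or when commit or the character's Overdrive check fails.
; It grants super armour, applies the buff, loops a heartbeat sound and spawns pose-copied ghost afterimages through a recursive WaitDelay.
; After a fixed delay, a closing montage ends Overdrive; hit-damage nodes are unconnected.
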(event Custom|AfterimageStart
  (bind _as_bp_katana_character_base (Variables|Default|GetAs%20BP%20Katana%20Character%20Base))
  (bind _mesh (Variables|/Script/Engine.Character|GetMesh _as_bp_katana_character_base))
  (Ability|Tasks|WaitDelay 0.1 :!label _label
    (:OnFinish
      (bind _returnvalue (Game|SpawnActorfromClass "/Game/SungSoo_Workspace/Blueprints/BP_PlayerGhostSpectrum.BP_PlayerGhostSpectrum_C" (Transformation|GetWorldTransform _mesh) "AlwaysSpawn" "OverrideRootScale" 0 0))
      (Class|PlayerGhostSpectrum|CopyPose _returnvalue _mesh (Variables|Default|GetNew%20Color))
      (goto _label))))

(event Ability|EventOnEndAbility
  (params (bWasCancelled :type Boolean)))

(event Ability|EventActivateAbility
  (bind _asbp_katana_character_base (Utilities|Casting|CastToBP_KatanaCharacterBase (Ability|GetAvatarActorfromActorInfo))
    (:then
      (Variables|Default|SetAs%20BP%20Katana%20Character%20Base _asbp_katana_character_base)
      (if (Animation|Montage|MontageIsPlaying (Components|SkeletalMesh|GetAnimInstance (Variables|/Script/Engine.Character|GetMesh (Variables|Default|GetAs%20BP%20Katana%20Character%20Base))) "/Game/Ju_Hyeong/Map/BP/ReMakeAnim/Basic_Character_Animation/Rolling/PlayerDash_Montage.PlayerDash_Montage")
        (Ability|CancelAbility :!label _label) ; 쿨타임 중이거나 비용이 없다면 어빌리티 취소
        (else
          (bind _returnvalue (Ability|CommitAbility))
          (if _returnvalue ; 쿨타임이 돌았거나 비용이 있다면!
            (bind _returnvalue_2 (Class|KatanaCharacterBase|CanOverDriveSkill (Variables|Default|GetAs%20BP%20Katana%20Character%20Base)))
            (if _returnvalue_2
              (Class|CharacterBase|SetHealth (Variables|Default|GetAs%20BP%20Katana%20Character%20Base) (- (Class|CharacterBase|GetHealth (Variables|Default|GetAs%20BP%20Katana%20Character%20Base)) (* (Class|CharacterBase|GetMaxHealth (Variables|Default|GetAs%20BP%20Katana%20Character%20Base)) 0.3)))
              (Utilities|Time|ClearandInvalidateTimerbyHandle (Variables|Default|GetSoundHandle))
              (Variables|/Script/GraduateProject.KatanaCharacterBase|SetbSpecialSkillSuperArmour (Variables|Default|GetAs%20BP%20Katana%20Character%20Base) true)
              (|PlayMontageandWaitProxy "None" (Variables|Default|GetMontage%20to%20Start%20Play) 1.0 "None" true 1.0 0.0
                (:then
                  (CallFunction|AfterimageStart)
                  (Class|KatanaCharacterBase|OnOverDriveBegin (Variables|Default|GetAs%20BP%20Katana%20Character%20Base))
                  (GameplayEffects|ApplyGameplayEffectSpecToSelf (Ability|GetAbilitySystemComponent (Variables|Default|GetAs%20BP%20Katana%20Character%20Base)) (GameplayEffects|MakeOutgoingSpec (Ability|GetAbilitySystemComponent (Variables|Default|GetAs%20BP%20Katana%20Character%20Base)) "/Game/Ju_Hyeong/GameEffect/overdrive/GE_OverDrive_StrengthAndAttackSpeedBuff.GE_OverDrive_StrengthAndAttackSpeedBuff_C" 0.0 (GameplayEffects|MakeEffectContext (Ability|GetAbilitySystemComponent (Variables|Default|GetAs%20BP%20Katana%20Character%20Base)))))
                  (bind _returnvalue_3 (Utilities|Time|SetTimerbyFunctionName 0 "PlayTickSound" 0.99 true))
                  (Variables|Default|SetSoundHandle _returnvalue_3)
                  (Utilities|FlowControl|Delay 15.0)
                  (|PlayMontageandWaitProxy "None" (Variables|Default|GetMontage%20to%20Play) 1.0 "None" true 1.0 0.0
                    (:OnCompleted
                      _)
                    (:OnBlendOut
                      _)
                    (:OnInterrupted
                      _)
                    (:OnCancelled
                      _))
                  (Class|KatanaCharacterBase|OnOverDriveEnd (Variables|Default|GetAs%20BP%20Katana%20Character%20Base))
                  (Variables|/Script/GraduateProject.KatanaCharacterBase|SetbSpecialSkillSuperArmour (Variables|Default|GetAs%20BP%20Katana%20Character%20Base) false)
                  (Ability|EndAbility)))
              (else
                (goto _label)))
            (else
              (goto _label))))))
    (:CastFailed
      (goto _label))))

(fn PlayTickSound
  (Audio|PlaySoundatLocation "/Game/Ju_Hyeong/Heart_beating_2.Heart_beating_2" (Transformation|GetActorLocation (Variables|Default|GetAs%20BP%20Katana%20Character%20Base)) "0, 0, 0" 1.0 1.0 0.0 0 0 0 0))