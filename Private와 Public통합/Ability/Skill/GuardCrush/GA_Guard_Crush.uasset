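; Guard Crush gameplay ability for the katana character: a hold-to-charge skill that deals direct guard damage.
; Activation plays a charge montage while a self-recalling delay loop raises the clamped damage multiplier.
; Release plays the attack montage, then the hit event applies guard damage via SetByCaller, plus the character's optional additional effect.
; A hit-reaction montage check at each stage resets the charge and ends the ability.
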(event Custom|StateCharging
  ;[1 1 1] 대미지 차징
  (Utilities|FalseGuardBreak
    (:else
      (if (stale Ability|EventActivateAbility _output_get_2)
        (Variables|Default|SetGuardBreakDamage (Math|Float|Clamp(Float) (+ (Variables|Default|GetGuardBreakDamage) 0.0225) 0.1))
        (Utilities|FlowControl|Delay 0.05)
        (CallFunction|StateCharging)))))

(event Ability|EventActivateAbility
  (bind _returnvalue (Ability|CommitAbility))
  (if _returnvalue ; 쿨타임이 돌았거나 비용이 있다면!
    (bind _asbp_katana_character_base (Utilities|Casting|CastToBP_KatanaCharacterBase (Ability|GetAvatarActorfromActorInfo))
      (:then
        (bind _output_get (Variables|Default|SetAs%20BP%20Katana%20Character%20Base _asbp_katana_character_base))
        (Utilities|FalseGuardBreak
          (:else
            (Class|KatanaCharacterBase|DirectionCameraLookingat _output_get)
            (Class|KatanaCharacterBase|PlayNoneSuperArmourSkillState (Variables|Default|GetAs%20BP%20Katana%20Character%20Base))
            (|PlayMontageandWaitProxy "None" (Variables|Default|GetMontage%20to%20Play) 1.0 "None" true 1.0 0.0
              (:then
                ;[1 1 1] 대미지 차징
                (Variables|Default|SetGuardBreakDamage 0.1)
                (bind _output_get_2 (Variables|Default|SetIsCharging true))
                (if _output_get_2
                  (Variables|Default|SetGuardBreakDamage (Math|Float|Clamp(Float) (+ (Variables|Default|GetGuardBreakDamage) 0.0225) 0.1))
                  (Utilities|FlowControl|Delay 0.05)
                  (CallFunction|StateCharging)))))))
      (:CastFailed
        (Ability|CancelAbility :!label _label) ; 쿨타임 중이거나 비용이 없다면 어빌리티 취소
      ))
    (else
      (goto _label))))

(event EventOnInputButtonReleased
  (params (Handle :type Gameplay%20Ability%20Spec%20Handle%20Structure%20%28by%20ref%29) (ActivationInfo :type Gameplay%20Ability%20Activation%20Info%20Structure%20%28by%20ref%29))
  (bind _as_bp_katana_character_base (Variables|Default|GetAs%20BP%20Katana%20Character%20Base))
  (bind _additionalattackeffectontarget (Variables|/Script/GraduateProject.CharacterBase|GetAdditionalAttackEffectOnTarget _as_bp_katana_character_base))
  (if (not (Utilities|AttackAnimCheak))
    (Utilities|FalseGuardBreak
      (:else
        (|PlayMontageandWaitProxy "None" (Variables|Default|GetMontage%20to%20Play_Attack) 1.0 "None" true 1.0 0.0
          (:then
            (bind _payload (Ability|Tasks|WaitGameplayEvent "(TagName=\"Event.Player.Ability.Hit\")" 0)
              (:then
                (Variables|Default|SetIsCharging false))
              (:EventReceived
                (Variables|Default|SetIsCharging false)
                (bind _returnvalue (Ability|GameplayEffect|AssignTagSetbyCallerMagnitude (Ability|MakeOutgoingGameplayEffectSpec "/Game/Ju_Hyeong/Example_SkillMana/DefenseDamage/GE_DirectDamageToGuard.GE_DirectDamageToGuard_C") "(TagName=\"Data.DamageMult\")" (Variables|Default|GetGuardBreakDamage)))
                (GameplayEffects|ApplyGameplayEffectSpecToTarget _returnvalue (.TargetData (Utilities|Struct|BreakGameplayEventData _payload)))
                (Variables|Default|SetGuardBreakDamage 0.0)
                ;[1 1 1] 23.04.04 성수 추가내용
                (if (Utilities|IsValidClass _additionalattackeffectontarget)
                  (bind _returnvalue_2 (Ability|GameplayEffect|AssignTagSetbyCallerMagnitude (Ability|MakeOutgoingGameplayEffectSpec _additionalattackeffectontarget) "(TagName=\"Data.DamageMult\")" (.EventMagnitude (Utilities|Struct|BreakGameplayEventData _payload))))
                  (GameplayEffects|ApplyGameplayEffectSpecToTarget _returnvalue_2 (.TargetData (Utilities|Struct|BreakGameplayEventData _payload)))))))
          (:OnCompleted
            (Class|KatanaCharacterBase|StopSkillState (Variables|Default|GetAs%20BP%20Katana%20Character%20Base) :!label _label)
            (Ability|EndAbility))
          (:OnBlendOut
            (goto _label))
          (:OnInterrupted
            (goto _label))
          (:OnCancelled
            (goto _label)))))))