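; Fire wind skill actor in the FireDash ability folder that damages targets and sets them ablaze.
; It plays a fire spell sound at its location on BeginPlay.
; The parent class handles base damage, then the override applies the GE_State_Ablaze gameplay effect from the katana character's ability system component to the target's.
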(event EventBeginPlay
  (|CallParentFunction)
  (Audio|SpawnSoundatLocation "/Game/Assets_Sound/Player/Fire_Spell_13_Cue.Fire_Spell_13_Cue" (Transformation|GetActorLocation) "0, 0, 0" 1.0 1.0 0.0 0 0))

(event EventApplyDamagetoTarget
  (params (TargetActor :type Actor%20Object%20Reference))
  (bind _as_bp_katana_character_base (Variables|Default|GetAs%20BP%20Katana%20Character%20Base))
  (bind _returnvalue (Ability|GetAbilitySystemComponent _as_bp_katana_character_base))
  (|CallParentFunction TargetActor)
  (GameplayEffects|ApplyGameplayEffectSpecToTarget _returnvalue (GameplayEffects|MakeOutgoingSpec _returnvalue "/Game/SungSoo_Workspace/Blueprints/Effects/State/GE_State_Ablaze.GE_State_Ablaze_C" 0.0 (GameplayEffects|MakeEffectContext _returnvalue)) (Ability|GetAbilitySystemComponent TargetActor)))

(fn ConstructionScript
  (|CallParentFunction))