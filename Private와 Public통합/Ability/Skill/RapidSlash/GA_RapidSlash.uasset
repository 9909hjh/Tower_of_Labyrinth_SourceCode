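; Gameplay ability for the katana character's Rapid Slash skill.
; On a successful commit it calls the character's camera-direction turn, applies an invincibility effect, enters super-armour skill state and plays a montage.
; Any montage exit stops the skill state and ends the ability, while a failed commit or cast cancels it.
; Hit-event nodes for damage and additional on-target effects exist but are disconnected, so this graph deals no damage.
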(event Ability|EventActivateAbility
  (bind _returnvalue (Ability|CommitAbility))
  (if _returnvalue ; 쿨타임이 돌았거나 비용이 있다면!
    (bind _asbp_katana_character_base (Utilities|Casting|CastToBP_KatanaCharacterBase (Ability|GetAvatarActorfromActorInfo))
      (:then
        (bind _output_get (Variables|Default|SetAs%20BP%20Katana%20Character%20Base _asbp_katana_character_base))
        (Class|KatanaCharacterBase|DirectionCameraLookingat _output_get)
        (Ability|ApplyGameplayEffectSpecToOwner (Ability|MakeOutgoingGameplayEffectSpec "/Game/Ju_Hyeong/GameEffect/GE_Invincible_RapidSlash.GE_Invincible_RapidSlash_C"))
        (Class|KatanaCharacterBase|PlaySuperArmourSkillState (Variables|Default|GetAs%20BP%20Katana%20Character%20Base))
        (|PlayMontageandWaitProxy "None" (Variables|Default|GetMontage%20to%20Play) 1.0 "None" true 1.0 0.0
          (:OnCompleted
            _)
          (:OnBlendOut
            _)
          (:OnInterrupted
            _)
          (:OnCancelled
            _))
        (Class|KatanaCharacterBase|StopSkillState (Variables|Default|GetAs%20BP%20Katana%20Character%20Base))
        (Ability|EndAbility))
      (:CastFailed
        (Ability|CancelAbility :!label _label) ; 쿨타임 중이거나 비용이 없다면 어빌리티 취소
      ))
    (else
      (goto _label))))

(event Ability|EventOnEndAbility
  (params (bWasCancelled :type Boolean)))