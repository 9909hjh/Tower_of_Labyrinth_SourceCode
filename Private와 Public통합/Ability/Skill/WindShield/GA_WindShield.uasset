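; Wind Shield gameplay ability that gives the katana character a self-applied move speed and defense effect.
; Activation cancels if the dash montage is playing or the commit of cost and cooldown fails.
; Otherwise it plays sounds, attaches a Niagara wind effect to the mesh, applies the effect, then after a fixed delay destroys the visual and ends.
; Montage and hit-event damage nodes are left unconnected and never run.
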(event Ability|EventActivateAbility
  (bind _asbp_katana_character_base (Utilities|Casting|CastToBP_KatanaCharacterBase (Ability|GetAvatarActorfromActorInfo))
    (:then
      (Variables|Default|SetAs%20BP%20Katana%20Character%20Base _asbp_katana_character_base)
      (if (Animation|Montage|MontageIsPlaying (Components|SkeletalMesh|GetAnimInstance (Variables|/Script/Engine.Character|GetMesh (Variables|Default|GetAs%20BP%20Katana%20Character%20Base))) "/Game/Ju_Hyeong/Map/BP/ReMakeAnim/Basic_Character_Animation/Rolling/PlayerDash_Montage.PlayerDash_Montage")
        (Ability|CancelAbility :!label _label) ; 쿨타임 중이거나 비용이 없다면 어빌리티 취소
        (else
          (bind _returnvalue (Ability|CommitAbility))
          (if _returnvalue ; 쿨타임이 돌았거나 비용이 있다면!
            (CallFunction|WindEffect)
            (GameplayEffects|ApplyGameplayEffectSpecToSelf (Ability|GetAbilitySystemComponent (Variables|Default|GetAs%20BP%20Katana%20Character%20Base)) (GameplayEffects|MakeOutgoingSpec (Ability|GetAbilitySystemComponent (Variables|Default|GetAs%20BP%20Katana%20Character%20Base)) "/Game/Ju_Hyeong/GameEffect/windShield/GE_WindShield_MoveSpeedAndDefense.GE_WindShield_MoveSpeedAndDefense_C" 0.0 (GameplayEffects|MakeEffectContext (Ability|GetAbilitySystemComponent (Variables|Default|GetAs%20BP%20Katana%20Character%20Base)))))
            (Utilities|FlowControl|Delay 5.0)
            (Components|DestroyComponent (Variables|Default|GetWindNiagaraEffectProperty))
            (Ability|EndAbility)
            (else
              (goto _label))))))
    (:CastFailed
      (goto _label))))

(event Ability|EventOnEndAbility
  (params (bWasCancelled :type Boolean)))

(fn WindEffect
  (bind _as_bp_katana_character_base (Variables|Default|GetAs%20BP%20Katana%20Character%20Base))
  (for _array_element (Utilities|Array|MakeArray (Variables|Default|GetSound) (Variables|Default|GetSound_0) (Variables|Default|GetSound_1))
    (Audio|PlaySoundatLocation _array_element (Transformation|GetActorLocation _as_bp_katana_character_base) "0, 0, 0" 1.0 1.0 0.0 0 0 0 0))
  (bind _returnvalue (Niagara|SpawnSystemAttached "/Game/Ju_Hyeong/Effect/VFX/NS_SlashR_02_Custom.NS_SlashR_02_Custom" (Variables|/Script/Engine.Character|GetMesh _as_bp_katana_character_base) "None" "0.000000,0.000000,120.000000" "0, 0, 0" "SnapToTargetIncludingScale" true))
  (Variables|Default|SetWindNiagaraEffectProperty _returnvalue))