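; BP_DivineLight_Actor is the actor spawned for the Divine Light skill, extending a parent that handles tick damage.
; It plays a looping cast sound on begin, fading it out and playing an ending spell sound when destroyed.
; Each damage tick checks the katana character's montages, destroying the actor if the hit montage plays or the skill montage stops, then runs the parent's tick damage.
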(event EventBeginPlay
  (|CallParentFunction)
  (bind _returnvalue (Audio|SpawnSoundatLocation "/Game/Assets_Sound/Player/General_Cast_Loop_1_Cue.General_Cast_Loop_1_Cue" (Transformation|GetActorLocation) "0, 0, 0" 1.0 1.0 0.0 0 0))
  (Variables|Default|SetSfxRef _returnvalue))

(event EventDestroyed
  (bind _sfxref (Variables|Default|GetSfxRef))
  (Utilities|IsValid _sfxref
    (:Is%20Valid
      (Audio|Components|Audio|FadeOut _sfxref 2.0 0.0 "Logarithmic" :!class /Script/Engine.AudioComponent)
      (Audio|SpawnSoundatLocation "/Game/Assets_Sound/Player/Arcane_Spell_12_4.Arcane_Spell_12_4" (Transformation|GetActorLocation) "0, 0, 0" 1.0 1.0 0.0 0 0))))

(event EventTickDamage
  (bind _as_bp_katana_character_base (Variables|Default|GetAs%20BP%20Katana%20Character%20Base))
  (bind _mesh (Variables|/Script/Engine.Character|GetMesh _as_bp_katana_character_base))
  (bind _returnvalue (Components|SkeletalMesh|GetAnimInstance _mesh))
  (Utilities|FlowControl|Sequence
    (:then_0
      (if (Animation|Montage|MontageIsPlaying _returnvalue "/Game/Ju_Hyeong/Map/BP/ReMakeAnim/Basic_Character_Animation/HitAnim/PlayerCharacter_SetHit_Montage.PlayerCharacter_SetHit_Montage")
        (Actor|DestroyActor :!label _label)
        (elif (not (Animation|Montage|MontageIsPlaying _returnvalue "/Game/Ju_Hyeong/Map/BP/ReMakeAnim/SkillAnim/DivineLight/DivineLight_Skill_Montage.DivineLight_Skill_Montage"))
          (goto _label))))
    (:then_1
      (|CallParentFunction))))

(fn ConstructionScript
  (|CallParentFunction))