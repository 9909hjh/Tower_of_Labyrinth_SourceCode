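; Sylph's Protection Gameplay Ability for the katana character: a self-buff to move speed and defense.
; It cancels if the dash montage is playing or the commit fails.
; Otherwise it starts a montage, immediately spawns the protection actor at the character's transform, applies the buff effect, and ends after a fixed delay.
; The hit-event damage logic, with SetByCaller magnitude and an optional extra effect, is disconnected and never runs.
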(event Ability|EventActivateAbility
  (bind _asbp_katana_character_base (Utilities|Casting|CastToBP_KatanaCharacterBase (Ability|GetAvatarActorfromActorInfo))
    (:then
      (Variables|Default|SetAs%20BP%20Katana%20Character%20Base _asbp_katana_character_base)
      (if (Animation|Montage|MontageIsPlaying (Components|SkeletalMesh|GetAnimInstance (Variables|/Script/Engine.Character|GetMesh (Variables|Default|GetAs%20BP%20Katana%20Character%20Base))) "/Game/Ju_Hyeong/Map/BP/ReMakeAnim/Basic_Character_Animation/Rolling/PlayerDash_Montage.PlayerDash_Montage")
        (Ability|CancelAbility :!label _label) ; 쿨타임 중이거나 비용이 없다면 어빌리티 취소
        (else
          (bind _returnvalue (Ability|CommitAbility))
          (if _returnvalue ; 쿨타임이 돌았거나 비용이 있다면!
            (|PlayMontageandWaitProxy "None" (Variables|Default|GetMontage%20to%20Play) 1.0 "None" true 1.0 0.0
              (:then
                (Game|SpawnActorfromClass "/Game/Ju_Hyeong/Ability/Skill/SylphsProtection/BP_SylphsProtection_Actor.BP_SylphsProtection_Actor_C" (Transformation|GetActorTransform (Variables|Default|GetAs%20BP%20Katana%20Character%20Base)) "Undefined" "OverrideRootScale" 0 0)
                (GameplayEffects|ApplyGameplayEffectSpecToSelf (Ability|GetAbilitySystemComponent (Variables|Default|GetAs%20BP%20Katana%20Character%20Base)) (GameplayEffects|MakeOutgoingSpec (Ability|GetAbilitySystemComponent (Variables|Default|GetAs%20BP%20Katana%20Character%20Base)) "/Game/Ju_Hyeong/GameEffect/SylphsProtection/GE_SylphsProtection_MoveSpeedAndDefense.GE_SylphsProtection_MoveSpeedAndDefense_C" 0.0 (GameplayEffects|MakeEffectContext (Ability|GetAbilitySystemComponent (Variables|Default|GetAs%20BP%20Katana%20Character%20Base)))))
                (Utilities|FlowControl|Delay 1e+01)
                (Ability|EndAbility)))
            (else
              (goto _label))))))
    (:CastFailed
      (goto _label))))

(event Ability|EventOnEndAbility
  (params (bWasCancelled :type Boolean)))