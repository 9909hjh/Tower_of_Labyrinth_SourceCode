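; Gameplay ability for the katana character's guard skill, which applies an invincibility effect and plays a montage.
; It cancels if the avatar cast fails, the dash montage is playing, or CommitAbility fails on cooldown or cost.
; Otherwise it calls DirectionCameraLookingAt, applies GE_Invincible_Guard to the owner, and ends when the montage completes, blends out or is stopped.
; Hit-event damage nodes, including an additional on-target effect, are present but unconnected.
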(event Ability|EventActivateAbility
  (bind _asbp_katana_character_base (Utilities|Casting|CastToBP_KatanaCharacterBase (Ability|GetAvatarActorfromActorInfo))
    (:then
      (Variables|Default|SetAs%20BP%20Katana%20Character%20Base _asbp_katana_character_base)
      (if (Animation|Montage|MontageIsPlaying (Components|SkeletalMesh|GetAnimInstance (Variables|/Script/Engine.Character|GetMesh (Variables|Default|GetAs%20BP%20Katana%20Character%20Base))) "/Game/Ju_Hyeong/Map/BP/ReMakeAnim/Basic_Character_Animation/Rolling/PlayerDash_Montage.PlayerDash_Montage")
        (Ability|CancelAbility :!label _label) ; 쿨타임 중이거나 비용이 없다면 어빌리티 취소
        (else
          (bind _returnvalue (Ability|CommitAbility))
          (if _returnvalue ; 쿨타임이 돌았거나 비용이 있다면!
            (Class|KatanaCharacterBase|DirectionCameraLookingat (Variables|Default|GetAs%20BP%20Katana%20Character%20Base))
            (Ability|ApplyGameplayEffectSpecToOwner (Ability|MakeOutgoingGameplayEffectSpec "/Game/Ju_Hyeong/GameEffect/GE_Invincible_Guard.GE_Invincible_Guard_C"))
            (|PlayMontageandWaitProxy "None" (Variables|Default|GetMontage%20to%20Play) 1.0 "None" true 1.0 0.0
              (:OnCompleted
                _)
              (:OnBlendOut
                _)
              (:OnInterrupted
                _)
              (:OnCancelled
                _))
            (Ability|EndAbility)
            (else
              (goto _label))))))
    (:CastFailed
      (goto _label))))

(event Ability|EventOnEndAbility
  (params (bWasCancelled :type Boolean)))