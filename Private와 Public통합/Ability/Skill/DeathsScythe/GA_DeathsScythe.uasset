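; GA_DeathsScythe is the Gameplay Ability for the katana character's Death's Scythe skill.
; On activation it commits, spawns BP_DeathsScythe_Actor at the avatar's transform with the avatar as Instigator, then ends immediately.
; It cancels if the commit or character cast fails.
; Leftover hit-event nodes for applying GE_Apply_Damage and the character's additional attack effect are disconnected, so this ability applies no damage itself.
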(event Ability|EventActivateAbility
  (bind _returnvalue (Ability|CommitAbility))
  (if _returnvalue ; 쿨타임이 돌았거나 비용이 있다면!
    (bind _asbp_katana_character_base (Utilities|Casting|CastToBP_KatanaCharacterBase (Ability|GetAvatarActorfromActorInfo))
      (:then
        (bind _output_get (Variables|Default|SetAs%20BP%20Katana%20Character%20Base _asbp_katana_character_base))
        (Game|SpawnActorfromClass "/Game/Ju_Hyeong/Ability/Skill/DeathsScythe/BP_DeathsScythe_Actor.BP_DeathsScythe_Actor_C" (Transformation|GetActorTransform _output_get) "Undefined" 0 _output_get)
        (Ability|EndAbility))
      (:CastFailed
        (Ability|CancelAbility :!label _label) ; 쿨타임 중이거나 비용이 없다면 어빌리티 취소
      ))
    (else
      (goto _label))))

(event Ability|EventOnEndAbility
  (params (bWasCancelled :type Boolean)))