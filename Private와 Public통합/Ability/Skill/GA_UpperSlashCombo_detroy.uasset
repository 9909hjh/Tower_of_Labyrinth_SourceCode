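; Gameplay ability for an upper slash skill that plays a montage and damages targets it hits.
; After committing, it starts the montage at the "Downer" section if the avatar CharacterBase is falling, otherwise at "Upper".
; A hit gameplay event supplies target data and a magnitude, passed as a SetByCaller damage multiplier into GE_Apply_Damage.
; The ability ends with the montage and cancels if commit or cast fails.
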(event Ability|EventActivateAbility
  (bind _returnvalue (Ability|CommitAbility))
  (if _returnvalue ; 쿨타임이 돌았거나 비용이 있다면!
    (bind _ascharacter_base (Utilities|Casting|CastToCharacterBase (Ability|GetAvatarActorfromActorInfo))
      (:then
        (bind _output_get (Variables|Default|SetAs%20Character%20Base _ascharacter_base))
        (if (AI|Components|NavMovement|IsFalling (Variables|/Script/Engine.Character|GetCharacterMovement _output_get))
          (Variables|Default|SetStart%20Section "Downer")
          (else
            (Variables|Default|SetStart%20Section "Upper")))
        (|PlayMontageandWaitProxy "None" (Variables|Default|GetMontage%20to%20Play) 1.0 (Variables|Default|GetStart%20Section) true 1.0 0.0
          (:then
            (bind _payload (Ability|Tasks|WaitGameplayEvent "(TagName=\"Event.Player.Ability.Hit\")" 0)
              (:EventReceived
                (bind _returnvalue_2 (Ability|GameplayEffect|AssignTagSetbyCallerMagnitude (Ability|MakeOutgoingGameplayEffectSpec "/Game/SungSoo_Workspace/Blueprints/Effects/GE_Apply_Damage.GE_Apply_Damage_C") "(TagName=\"Data.DamageMult\")" (.EventMagnitude (Utilities|Struct|BreakGameplayEventData _payload))))
                (GameplayEffects|ApplyGameplayEffectSpecToTarget _returnvalue_2 (.TargetData (Utilities|Struct|BreakGameplayEventData _payload))))))
          (:OnCompleted
            (Ability|EndAbility :!label _label))
          (:OnBlendOut
            (goto _label))
          (:OnInterrupted
            (goto _label))
          (:OnCancelled
            (goto _label))))
      (:CastFailed
        (Ability|CancelAbility :!label _label_2) ; 쿨타임 중이거나 비용이 없다면 어빌리티 취소
      ))
    (else
      (goto _label_2))))

(event Ability|EventOnEndAbility
  (params (bWasCancelled :type Boolean)))