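; Hit actor for the Dragon Breath skill that deals repeated area damage and sets targets ablaze.
; Each tick box-traces for pawns at its location and rotation, ignoring the katana character, then damages hits and spawns hit effects and camera shake.
; Damage extends the parent logic by applying the Ablaze GameplayEffect through GAS.
; TickDamage re-calls itself on an evenly divided delay until its counter runs out, then destroys the actor after a delay.
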(event EventApplyDamagetoTarget
  (params (TargetActor :type Actor%20Object%20Reference))
  (bind _as_bp_katana_character_base (Variables|Default|GetAs%20BP%20Katana%20Character%20Base))
  (bind _returnvalue (Ability|GetAbilitySystemComponent _as_bp_katana_character_base))
  (|CallParentFunction TargetActor)
  (GameplayEffects|ApplyGameplayEffectSpecToTarget _returnvalue (GameplayEffects|MakeOutgoingSpec _returnvalue "/Game/SungSoo_Workspace/Blueprints/Effects/State/GE_State_Ablaze.GE_State_Ablaze_C" 0.0 (GameplayEffects|MakeEffectContext _returnvalue)) (Ability|GetAbilitySystemComponent TargetActor)))

(event EventTickDamage
  (bind _returnvalue (Transformation|GetActorLocation))
  (if (> (Variables|Default|GetCrrentValue) 0.0)
    (Math|Float|DecrementFloat (Variables|Default|GetCrrentValue)
      (:%20%20
        (Utilities|FlowControl|Sequence
          (:then_0
            (CallFunction|OnPreTickDamage)
            (bind (_outhits _returnvalue_2) (Class|KismetSystemLibrary|BoxTraceMultiforObjects _returnvalue _returnvalue "500.000000,100.000000,100.000000" (Transformation|GetActorRotation) (Utilities|Array|MakeArray "ObjectTypeQuery3") false (Utilities|Array|MakeArray (Variables|Default|GetAs%20BP%20Katana%20Character%20Base)) "None" true))
            (if _returnvalue_2
              (for _array_element _outhits
                (Utilities|FlowControl|Sequence
                  (:then_0
                    (CallFunction|ApplyDamagetoTarget (.HitActor (Collision|BreakHitResult _array_element))))
                  (:then_1
                    ;[1 1 1] 히트 이펙트 스폰
                    (Class|GameplayHelperLibrary|SpawnHitEffects (Variables|Default|GetAs%20BP%20Katana%20Character%20Base) (.HitActor (Collision|BreakHitResult _array_element)) (Variables|Default|GetAttack%20Hit%20Sound) (Variables|Default|GetHit%20Vfx) "1.000000,1.000000,1.000000") ; HitResult는 트레이스 결과 값
                    (Camera|PlayWorldCameraShake (Variables|Default|GetShake) (Transformation|GetActorLocation) 0.0 3e+03))))))
          (:then_1
            (Utilities|FlowControl|Delay (/ (Variables|Default|GetForSecond) (Variables|Default|GetNumExecutions)))
            (CallFunction|TickDamage)))))
    (else
      (Utilities|FlowControl|Delay (Variables|Default|GetDelayDestroyActor))
      (Actor|DestroyActor))))

(fn ConstructionScript
  (|CallParentFunction))