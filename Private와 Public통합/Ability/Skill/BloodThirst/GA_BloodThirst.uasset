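; BloodThirst gameplay ability for the katana character, a timed self-buff with a health cost suggested by its effect names.
; Activation cancels during a dash montage or on failed commit; otherwise it plays a montage and applies a take-damage effect to the owner.
; Enemy-death events trigger a restore-health effect until the ability ends after about ten seconds.
; A looping timer plays stab sound and slash VFX, cleared only upon the next committed activation.
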(event Ability|EventActivateAbility
  (bind _asbp_katana_character_base (Utilities|Casting|CastToBP_KatanaCharacterBase (Ability|GetAvatarActorfromActorInfo))
    (:then
      (Variables|Default|SetAs%20BP%20Katana%20Character%20Base _asbp_katana_character_base)
      (if (Animation|Montage|MontageIsPlaying (Components|SkeletalMesh|GetAnimInstance (Variables|/Script/Engine.Character|GetMesh (Variables|Default|GetAs%20BP%20Katana%20Character%20Base))) "/Game/Ju_Hyeong/Map/BP/ReMakeAnim/Basic_Character_Animation/Rolling/PlayerDash_Montage.PlayerDash_Montage")
        (Ability|CancelAbility :!label _label) ; 쿨타임 중이거나 비용이 없다면 어빌리티 취소
        (else
          (bind _returnvalue (Ability|CommitAbility))
          (if _returnvalue ; 쿨타임이 돌았거나 비용이 있다면!
            (Utilities|Time|ClearandInvalidateTimerbyHandle (Variables|Default|GetTimerHandle))
            (|PlayMontageandWaitProxy "None" (Variables|Default|GetMontage%20to%20Play) 1.0 "None" true 1.0 0.0
              (:then
                (Utilities|FlowControl|Sequence
                  (:then_0
                    (bind _returnvalue_2 (Utilities|Time|SetTimerbyFunctionName 0 "PlayTickSound" 5.0 true))
                    (Variables|Default|SetTimerHandle _returnvalue_2)
                    (Ability|ApplyGameplayEffectSpecToOwner (Ability|MakeOutgoingGameplayEffectSpec "/Game/Ju_Hyeong/GameEffect/BloodThirst/GE_Weapon_BloodThirst_AdditionalEffect_TakeDamage.GE_Weapon_BloodThirst_AdditionalEffect_TakeDamage_C"))
                    (Ability|Tasks|WaitGameplayEvent "(TagName=\"Event.Enemy.Died\")" 0
                      (:EventReceived
                        (Ability|ApplyGameplayEffectSpecToOwner (Ability|MakeOutgoingGameplayEffectSpec "/Game/Ju_Hyeong/GameEffect/BloodThirst/GE_Weapon_BloodThirst_AdditionalEffect_RestoreHealth.GE_Weapon_BloodThirst_AdditionalEffect_RestoreHealth_C")))))
                  (:then_1
                    (Utilities|FlowControl|Delay 10.2)
                    (Ability|EndAbility)))))
            (else
              (goto _label))))))
    (:CastFailed
      (goto _label))))

(fn PlayTickSound
  (bind _as_bp_katana_character_base (Variables|Default|GetAs%20BP%20Katana%20Character%20Base))
  (bind _returnvalue (Transformation|GetActorLocation _as_bp_katana_character_base))
  (Audio|PlaySoundatLocation "/Game/Assets_Sound/Player/Dagger_Stab__Flesh__2.Dagger_Stab__Flesh__2" _returnvalue "0, 0, 0" 1.0 1.0 0.0 0 0 0 0)
  (Niagara|SpawnSystematLocation "/Game/Assets/Hack_And_Slash_FX/VFX_Niagara/Impacts/NS_Demon_Slash_Impact.NS_Demon_Slash_Impact" _returnvalue))