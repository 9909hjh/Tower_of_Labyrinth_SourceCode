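; Elemental Circle skill actor that sets up its magnitude and gameplay effect when spawned.
; On BeginPlay, after the parent's logic, it sets Magnitude to twice the Strength of the referenced katana character.
; It then randomly picks one of three GameplayEffect classes as its active effect.
; Overlap and Tick events are unused, and this graph does not itself apply the effect.
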(event EventBeginPlay
  (|CallParentFunction)
  (Variables|Default|SetMagnitude (* (Class|CharacterBase|GetStrength (Variables|Default|GetAs%20BP%20Katana%20Character%20Base)) 2.0))
  (Variables|Default|SetGameplay%20Effect%20Class (.OutItem (Utilities|Array|Random (Utilities|Array|MakeArray (Variables|Default|GetGameplay%20Effect%20Class_0) (Variables|Default|GetGameplay%20Effect%20Class_1) (Variables|Default|GetGameplay%20Effect%20Class_2))))))

(event Collision|EventActorBeginOverlap
  (params (OtherActor :type Actor%20Object%20Reference)))

(event EventTick
  (params (DeltaSeconds :type Float%20%28single-precision%29)))

(fn ConstructionScript
  (|CallParentFunction))