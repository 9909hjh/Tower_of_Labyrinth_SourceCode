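; GA_SalamandersProtection is a katana character ability granting a timed fire (Salamander) or ice (IceQueen) buff, chosen by FalseIceTureSalamander.
; Activation cancels during the dash montage or when commit fails; otherwise it calls the element's begin hook, plays sound, attaches body Niagara and applies a self GameplayEffect.
; After a fixed delay it calls the end hook, destroys the Niagara and ends.
; Montage and hit-event damage nodes remain unconnected.
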(event Ability|EventActivateAbility
  (bind _asbp_katana_character_base (Utilities|Casting|CastToBP_KatanaCharacterBase (Ability|GetAvatarActorfromActorInfo))
    (:then
      (Variables|Default|SetAs%20BP%20Katana%20Character%20Base _asbp_katana_character_base)
      (if (Animation|Montage|MontageIsPlaying (Components|SkeletalMesh|GetAnimInstance (Variables|/Script/Engine.Character|GetMesh (Variables|Default|GetAs%20BP%20Katana%20Character%20Base))) "/Game/Ju_Hyeong/Map/BP/ReMakeAnim/Basic_Character_Animation/Rolling/PlayerDash_Montage.PlayerDash_Montage")
        (Ability|CancelAbility :!label _label) ; 쿨타임 중이거나 비용이 없다면 어빌리티 취소
        (else
          (bind _returnvalue (Ability|CommitAbility))
          (if _returnvalue ; 쿨타임이 돌았거나 비용이 있다면!
            (CallFunction|ChaeckElementBegin (Variables|Default|GetAs%20BP%20Katana%20Character%20Base))
            (GameplayEffects|ApplyGameplayEffectSpecToSelf (Ability|GetAbilitySystemComponent (Variables|Default|GetAs%20BP%20Katana%20Character%20Base)) (GameplayEffects|MakeOutgoingSpec (Ability|GetAbilitySystemComponent (Variables|Default|GetAs%20BP%20Katana%20Character%20Base)) (Variables|Default|GetGameplay%20Effect%20Class) 0.0 (GameplayEffects|MakeEffectContext (Ability|GetAbilitySystemComponent (Variables|Default|GetAs%20BP%20Katana%20Character%20Base)))))
            (Utilities|FlowControl|Delay 1e+01)
            (CallFunction|ChaeckElementEnd (Variables|Default|GetAs%20BP%20Katana%20Character%20Base))
            (Ability|EndAbility)
            (else
              (goto _label))))))
    (:CastFailed
      (goto _label))))

(fn ChaeckElementBegin
  (params (타깃 :type Katana%20Character%20Base%20Object%20Reference))
  (if (Variables|Default|GetFalseIceTureSalamander)
    (Class|KatanaCharacterBase|OnSalamandersBegin 타깃)
    (Audio|PlaySoundatLocation "/Game/Assets_Sound/Player/Fire_Spell_2_Cue.Fire_Spell_2_Cue" (Transformation|GetActorLocation (Variables|Default|GetAs%20BP%20Katana%20Character%20Base)) "0, 0, 0" 1.0 1.0 0.0 0 0 0 0)
    (bind _returnvalue (Niagara|SpawnSystemAttached "/Game/Ju_Hyeong/Effect/VFX/NS_FlameBody_YT.NS_FlameBody_YT" (Variables|/Script/Engine.Character|GetMesh (Variables|Default|GetAs%20BP%20Katana%20Character%20Base)) "None" "0, 0, 0" "0, 0, 0" "SnapToTargetIncludingScale" true))
    (Variables|Default|SetElementEffect _returnvalue)
    (else
      (Class|KatanaCharacterBase|OnIceQueenBegin 타깃)
      (Audio|PlaySoundatLocation "/Game/Assets_Sound/Player/Wind_Spell_9_Cue.Wind_Spell_9_Cue" (Transformation|GetActorLocation (Variables|Default|GetAs%20BP%20Katana%20Character%20Base)) "0, 0, 0" 1.0 1.0 0.0 0 0 0 0)
      (bind _returnvalue_2 (Niagara|SpawnSystemAttached "/Game/Ju_Hyeong/Effect/VFX/NS_IceBody_YT.NS_IceBody_YT" (Variables|/Script/Engine.Character|GetMesh (Variables|Default|GetAs%20BP%20Katana%20Character%20Base)) "None" "0, 0, 0" "0, 0, 0" "SnapToTargetIncludingScale" true))
      (Variables|Default|SetElementEffect_Ice _returnvalue_2)))
  (return))

(fn ChaeckElementEnd
  (params (타깃 :type Katana%20Character%20Base%20Object%20Reference))
  (if (Variables|Default|GetFalseIceTureSalamander)
    (Class|KatanaCharacterBase|OnSalamandersEnd 타깃)
    (Components|DestroyComponent (Variables|Default|GetElementEffect))
    (else
      (Class|KatanaCharacterBase|OnIceQueenEnd 타깃)
      (Components|DestroyComponent (Variables|Default|GetElementEffect_Ice))))
  (return))