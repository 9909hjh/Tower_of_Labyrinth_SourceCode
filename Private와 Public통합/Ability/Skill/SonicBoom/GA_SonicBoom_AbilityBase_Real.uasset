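; GA_SonicBoom_AbilityBase_Real is a Gameplay Ability for the katana character's SonicBoom skill.
; After committing, it turns the character via DirectionCameraLookingAt, enters a super-armour state and plays a montage, locking yaw to controller rotation for blade skills.
; Hit gameplay events apply damage and optional additional effects to event targets, scaled by SetByCaller magnitude.
; Montage end or interruption restores state and ends the ability; failed commit or cast cancels it.
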(event Ability|EventActivateAbility
  (bind _as_character_base (Variables|Default|GetAs%20Character%20Base))
  (bind _additionalattackeffectontarget (Variables|/Script/GraduateProject.CharacterBase|GetAdditionalAttackEffectOnTarget _as_character_base))
  (bind _returnvalue (Ability|CommitAbility))
  (if _returnvalue ; 쿨타임이 돌았거나 비용이 있다면!
    (bind _asbp_katana_character_base (Utilities|Casting|CastToBP_KatanaCharacterBase (Ability|GetAvatarActorfromActorInfo))
      (:then
        (bind _output_get (Variables|Default|SetAs%20BP%20Katana%20Character%20Base _asbp_katana_character_base))
        (if (Variables|Default|GetBladeSkill?)
          (Variables|/Script/Engine.Pawn|SetbUseControllerRotationYaw _output_get true))
        (Class|KatanaCharacterBase|DirectionCameraLookingat _output_get)
        (Class|KatanaCharacterBase|PlaySuperArmourSkillState (Variables|Default|GetAs%20BP%20Katana%20Character%20Base))
        (|PlayMontageandWaitProxy "None" (Variables|Default|GetMontage%20to%20Play) 1.0 "None" true 1.0 0.0
          (:then
            (bind _payload (Ability|Tasks|WaitGameplayEvent "(TagName=\"Event.Player.Ability.Hit\")" 0)
              (:EventReceived
                (bind _returnvalue_2 (Ability|GameplayEffect|AssignTagSetbyCallerMagnitude (Ability|MakeOutgoingGameplayEffectSpec "/Game/SungSoo_Workspace/Blueprints/Effects/GE_Apply_Damage.GE_Apply_Damage_C") "(TagName=\"Data.DamageMult\")" (.EventMagnitude (Utilities|Struct|BreakGameplayEventData _payload))))
                (GameplayEffects|ApplyGameplayEffectSpecToTarget _returnvalue_2 (.TargetData (Utilities|Struct|BreakGameplayEventData _payload)))
                ;[1 1 1] 23.04.04 성수 추가내용
                (if (Utilities|IsValidClass _additionalattackeffectontarget)
                  (bind _returnvalue_3 (Ability|GameplayEffect|AssignTagSetbyCallerMagnitude (Ability|MakeOutgoingGameplayEffectSpec _additionalattackeffectontarget) "(TagName=\"Data.DamageMult\")" (.EventMagnitude (Utilities|Struct|BreakGameplayEventData _payload))))
                  (GameplayEffects|ApplyGameplayEffectSpecToTarget _returnvalue_3 (.TargetData (Utilities|Struct|BreakGameplayEventData _payload)))))))
          (:OnCompleted
            (Class|KatanaCharacterBase|StopSkillState (Variables|Default|GetAs%20BP%20Katana%20Character%20Base) :!label _label)
            (Variables|/Script/Engine.Pawn|SetbUseControllerRotationYaw (Variables|Default|GetAs%20BP%20Katana%20Character%20Base) false)
            (Ability|EndAbility))
          (:OnBlendOut
            (goto _label))
          (:OnInterrupted
            (goto _label))
          (:OnCancelled
            (goto _label))))
      (:CastFailed
        (Ability|CancelAbility :!label _label_2) ; 쿨타임 중이거나 비용이 없다면 어빌리티 취소
      ))
    (else
      (goto _label_2))))

(event Ability|EventOnEndAbility
  (params (bWasCancelled :type Boolean)))