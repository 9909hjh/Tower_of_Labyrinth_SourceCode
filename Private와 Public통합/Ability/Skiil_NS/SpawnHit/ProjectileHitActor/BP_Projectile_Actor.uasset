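; Skill hit actor for the katana player character that damages enemies overlapping its box, playing a spawn sound and destroying itself after a set delay.
; On overlap, the player's ability system applies a damage GameplayEffect with a set-by-caller multiplier to the enemy.
; It optionally adds an elemental effect, then spawns hit sound and VFX.
; Miss-feedback and hit-event logic are present but unconnected.
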(event OnComponentBeginOverlap(Box)
  (params (OverlappedComponent :type Primitive%20Component%20Object%20Reference) (OtherActor :type Actor%20Object%20Reference) (OtherComp :type Primitive%20Component%20Object%20Reference) (OtherBodyIndex :type Integer) (bFromSweep :type Boolean) (SweepResult :type Hit%20Result%20Structure%20%28by%20ref%29))
  (bind _hitactor (Collision|BreakHitResult SweepResult))
  (bind _as_bp_katana_character_base (Variables|Default|GetAs%20BP%20Katana%20Character%20Base))
  (bind _as_bp_katana_character_base_2 (Variables|Default|GetAs%20BP%20Katana%20Character%20Base))
  (bind _returnvalue (Ability|GetAbilitySystemComponent _as_bp_katana_character_base))
  (bind _returnvalue_2 (Ability|GetAbilitySystemComponent _as_bp_katana_character_base_2))
  (bind _asenemy_character_base (Utilities|Casting|CastToEnemyCharacterBase _hitactor))
  (Utilities|FlowControl|Sequence
    (:then_0
      (bind _returnvalue_3 (Ability|GameplayEffect|AssignTagSetbyCallerMagnitude (GameplayEffects|MakeOutgoingSpec _returnvalue "/Game/SungSoo_Workspace/Blueprints/Effects/GE_Apply_Damage.GE_Apply_Damage_C" 0.0 (GameplayEffects|MakeEffectContext _returnvalue)) "(TagName=\"Data.DamageMult\")" (Variables|Default|GetMagnitude)))
      (GameplayEffects|ApplyGameplayEffectSpecToTarget _returnvalue _returnvalue_3 (Ability|GetAbilitySystemComponent _asenemy_character_base)))
    (:then_1
      ;[1 1 1] 속성공격
      (if (Variables|속성공격|GetElemental)
        (GameplayEffects|ApplyGameplayEffectSpecToTarget _returnvalue_2 (GameplayEffects|MakeOutgoingSpec _returnvalue_2 (Variables|속성공격|GetGameplay%20Effect%20Class) 0.0 (GameplayEffects|MakeEffectContext _returnvalue_2)) (Ability|GetAbilitySystemComponent _asenemy_character_base))))
    (:then_2
      ;[1 1 1] 히트 성공 사운드
      (Class|GameplayHelperLibrary|SpawnHitEffects (Variables|Default|GetAs%20BP%20Katana%20Character%20Base) _hitactor (Variables|SFXVFX|GetAttack%20Success%20Hit%20Sound) (Variables|SFXVFX|GetAttack%20Success%20Hit%20Vfx) (Variables|SFXVFX|GetVfx%20Scale%20Vector)))))

(event EventBeginPlay
  (bind _asbp_katana_character_base (Utilities|Casting|CastToBP_KatanaCharacterBase (Game|Player|GetPlayerPawn 0)))
  (Variables|Default|SetAs%20BP%20Katana%20Character%20Base _asbp_katana_character_base)
  (Audio|PlaySoundatLocation (Variables|SFXVFX|GetSpawnAttackSound) (Transformation|GetActorLocation) "0, 0, 0" 1.0 1.0 0.0 0 0 0 0)
  (Utilities|FlowControl|Delay (Variables|Default|GetDelayDestroyActor))
  (Actor|DestroyActor))

(fn ConstructionScript)