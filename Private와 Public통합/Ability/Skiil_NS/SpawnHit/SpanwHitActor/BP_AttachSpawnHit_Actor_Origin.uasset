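; Base area-hit skill actor that deals repeated damage around itself, optionally snapping to the player katana character's capsule.
; BeginPlay plays a spawn sound, starts a Delay-driven recursive TickDamage loop and schedules self-destruction.
; Each tick calls the overridable OnPreTickDamage, then sphere-traces pawns, applying a SetByCaller GAS damage effect, hit effects and camera shake.
; Older timer-based loop and gameplay-event nodes remain unconnected.
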(event Custom|OnPreTickDamage
  ;[1 1 1] 2023-05-13 성수 추가, 죽음의 낫 스킬 등에서 오버라이드
)

(event Custom|ApplyDamageToTarget
  (params (TargetActor :type Actor%20Object%20Reference))
  (bind _as_bp_katana_character_base (Variables|Default|GetAs%20BP%20Katana%20Character%20Base))
  (bind _returnvalue (Ability|GetAbilitySystemComponent _as_bp_katana_character_base))
  ;[1 1 1] 23-05-14 성수가 로직 수정
  (bind _returnvalue_2 (Ability|GameplayEffect|AssignTagSetbyCallerMagnitude (GameplayEffects|MakeOutgoingSpec _returnvalue "/Game/SungSoo_Workspace/Blueprints/Effects/GE_Apply_Damage.GE_Apply_Damage_C" 0.0 (GameplayEffects|MakeEffectContext _returnvalue)) "(TagName=\"Data.DamageMult\")" (Variables|Default|GetAddDamageValue)))
  (bind _returnvalue_3 (Ability|GameplayEffect|AssignTagSetbyCallerMagnitude _returnvalue_2 "(TagName=\"Data.FinalDamageRate\")" (Variables|Default|GetFinalDamageRate)))
  (GameplayEffects|ApplyGameplayEffectSpecToTarget _returnvalue _returnvalue_3 (Ability|GetAbilitySystemComponent TargetActor)))

(event Custom|TickDamage
  (bind _returnvalue (Transformation|GetActorLocation))
  (if (> (Variables|공격횟수|GetCrrentValue) 0.0)
    (Math|Float|DecrementFloat (Variables|공격횟수|GetCrrentValue)
      (:%20%20
        (Utilities|FlowControl|Sequence
          (:then_0
            (CallFunction|OnPreTickDamage)
            (bind (_outhits _returnvalue_2) (Collision|MultiSphereTraceForObjects _returnvalue _returnvalue (Variables|Default|GetRadius) (Utilities|Array|MakeArray "ObjectTypeQuery3") false (Utilities|Array|MakeArray (Variables|Default|GetAs%20BP%20Katana%20Character%20Base)) "None"))
            (if _returnvalue_2
              (for _array_element _outhits
                (Utilities|FlowControl|Sequence
                  (:then_0
                    (CallFunction|ApplyDamagetoTarget (.HitActor (Collision|BreakHitResult _array_element))))
                  (:then_1
                    ;[1 1 1] 히트 이펙트 스폰
                    (Class|GameplayHelperLibrary|SpawnHitEffects (Variables|Default|GetAs%20BP%20Katana%20Character%20Base) (.HitActor (Collision|BreakHitResult _array_element)) (Variables|SFX,VFX|GetAttack%20Hit%20Sound) (Variables|SFX,VFX|GetHit%20Vfx) "1.000000,1.000000,1.000000") ; HitResult는 트레이스 결과 값
                    (Camera|PlayWorldCameraShake (Variables|Default|GetShake) (Transformation|GetActorLocation) 0.0 3e+03))))))
          (:then_1
            (Utilities|FlowControl|Delay (/ (Variables|공격횟수|GetForSecond) (Variables|공격횟수|GetNumExecutions)))
            (CallFunction|TickDamage)))))
    (else
      (Utilities|FlowControl|Delay (Variables|Default|GetDelayDestroyActor))
      (Actor|DestroyActor))))

(event EventBeginPlay
  (bind _asbp_katana_character_base (Utilities|Casting|CastToBP_KatanaCharacterBase (Game|Player|GetPlayerPawn 0)))
  (bind _output_get (Variables|Default|SetAs%20BP%20Katana%20Character%20Base _asbp_katana_character_base))
  (Utilities|FlowControl|Sequence
    (:then_0
      ;[1 1 1] 23-05-14 성수 추가
      (if (Variables|Default|GetbAttached?)
        (Transformation|AttachComponentToComponent (Variables|Default|GetScene) (Variables|/Script/Engine.Character|GetCapsuleComponent _output_get) "None" "SnapToTarget" "KeepRelative" "KeepRelative" true)))
    (:then_1
      (Audio|PlaySoundatLocation (Variables|SFX,VFX|GetSpawnAttackSound) (Transformation|GetActorLocation) "0, 0, 0" 1.0 1.0 0.0 0 0 0 0)
      (Variables|공격횟수|SetCrrentValue (Variables|공격횟수|GetNumExecutions))
      ;[1 1 1] 230513 성수가 로직 수정 (타이머 X 방식)
      (CallFunction|TickDamage)
      ;[1 1 1] 참고: 15초 이상 지속되는 장판기가 있다면 InitialLifeSpan 값 수정 필요
      (Utilities|FlowControl|Delay (Variables|Default|GetDelayDestroyActor))
      (Actor|DestroyActor))))

(fn ConstructionScript)