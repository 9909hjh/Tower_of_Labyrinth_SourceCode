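; Spawned skill hit-box actor that deals repeated area damage on behalf of the player's katana character.
; BeginPlay plays a sound, starts a timer spacing damage ticks at ForSecond/NumExecutions, and destroys the actor after a delay.
; Each tick shakes the camera and box-traces pawns, applying GAS damage with a SetByCaller multiplier, an optional elemental effect and hit effects.
; The timer clears when a hitting tick finds the count used up.
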(event Custom|TickDamage
  (bind _returnvalue (Transformation|GetActorLocation))
  (bind _as_bp_katana_character_base (Variables|Default|GetAs%20BP%20Katana%20Character%20Base))
  (bind _as_bp_katana_character_base_2 (Variables|Default|GetAs%20BP%20Katana%20Character%20Base))
  (bind _returnvalue_2 (Ability|GetAbilitySystemComponent _as_bp_katana_character_base))
  (bind _returnvalue_3 (Ability|GetAbilitySystemComponent _as_bp_katana_character_base_2))
  (Utilities|FlowControl|Sequence
    (:then_0
      (Camera|PlayWorldCameraShake (Variables|Default|GetShake) (Transformation|GetActorLocation) 0.0 5e+03))
    (:then_1
      (bind (_outhits _returnvalue_4) (Class|KismetSystemLibrary|BoxTraceMultiforObjects _returnvalue _returnvalue (Variables|Default|GetHalf%20Size) (Transformation|GetActorRotation) (Utilities|Array|MakeArray "ObjectTypeQuery3") false (Utilities|Array|MakeArray (Variables|Default|GetAs%20BP%20Katana%20Character%20Base)) "None" true))
      (Variables|공격횟수|SetCrrentValue (- (Variables|공격횟수|GetCrrentValue) 1.0))
      (if _returnvalue_4
        (for _array_element _outhits
          (Utilities|FlowControl|Sequence
            (:then_0
              (bind _returnvalue_5 (Ability|GameplayEffect|AssignTagSetbyCallerMagnitude (GameplayEffects|MakeOutgoingSpec _returnvalue_2 "/Game/SungSoo_Workspace/Blueprints/Effects/GE_Apply_Damage.GE_Apply_Damage_C" 0.0 (GameplayEffects|MakeEffectContext _returnvalue_2)) "(TagName=\"Data.DamageMult\")" (Variables|Default|GetAddDamageValue)))
              (GameplayEffects|ApplyGameplayEffectSpecToTarget _returnvalue_2 _returnvalue_5 (Ability|GetAbilitySystemComponent (.HitActor (Collision|BreakHitResult _array_element)))))
            (:then_1
              ;[1 1 1] 속성공격
              (if (Variables|속성공격|GetElemental)
                (GameplayEffects|ApplyGameplayEffectSpecToTarget _returnvalue_3 (GameplayEffects|MakeOutgoingSpec _returnvalue_3 (Variables|속성공격|GetGameplay%20Effect%20Class) 0.0 (GameplayEffects|MakeEffectContext _returnvalue_3)) (Ability|GetAbilitySystemComponent (.HitActor (Collision|BreakHitResult _array_element))))))
            (:then_2
              ;[1 1 1] 히트 이펙트 스폰
              (Class|GameplayHelperLibrary|SpawnHitEffects (Variables|Default|GetAs%20BP%20Katana%20Character%20Base) (.HitActor (Collision|BreakHitResult _array_element)) (Variables|SFX,VFX|GetAttack%20Hit%20Sound) (Variables|SFX,VFX|GetHit%20Vfx) "1.000000,1.000000,1.000000") ; HitResult는 트레이스 결과 값
            )))
        ;[1 1 1] 클리어 및 삭제
        (if (<= (Variables|공격횟수|GetCrrentValue) 0.0)
          (Utilities|Time|ClearandInvalidateTimerbyHandle (Variables|Default|GetSpawnTimerHandle))
          (Utilities|FlowControl|Delay (Variables|Default|GetDelayDestroyActor))
          (Actor|DestroyActor))))))

(event EventBeginPlay
  (bind _asbp_katana_character_base (Utilities|Casting|CastToBP_KatanaCharacterBase (Game|Player|GetPlayerPawn 0)))
  (Variables|Default|SetAs%20BP%20Katana%20Character%20Base _asbp_katana_character_base)
  (Audio|PlaySoundatLocation (Variables|SFX,VFX|GetSpawnAttackSound) (Transformation|GetActorLocation) "0, 0, 0" 1.0 1.0 0.0 0 0 0 0)
  (Variables|공격횟수|SetCrrentValue (Variables|공격횟수|GetNumExecutions))
  (bind _returnvalue (Utilities|Time|SetTimerbyEvent (delegate Custom|TickDamage) (/ (Variables|공격횟수|GetForSecond) (Variables|공격횟수|GetNumExecutions)) (Variables|공격횟수|GetLooping)))
  (Variables|Default|SetSpawnTimerHandle _returnvalue)
  (Utilities|FlowControl|Delay (Variables|Default|GetDelayDestroyActor))
  (Actor|DestroyActor))

(fn ConstructionScript)