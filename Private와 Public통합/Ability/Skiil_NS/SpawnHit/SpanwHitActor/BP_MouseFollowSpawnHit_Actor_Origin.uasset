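; Skill hit actor that follows the katana player character and control rotation each frame, dealing repeated area damage.
; On BeginPlay it plays a sound, then TickDamage re-calls itself through Delay, spreading NumExecutions box traces over ForSecond before destroying the actor, also capped by DelayDestroyActor.
; Each pawn hit receives a GAS damage effect with SetByCaller magnitudes, plus hit effects and camera shake.
; An older timer setup remains unconnected.
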(event Custom|ApplyDamageToTarget
  (params (TargetActor :type Actor%20Object%20Reference))
  (bind _as_bp_katana_character_base (Variables|Default|GetAs%20BP%20Katana%20Character%20Base))
  (bind _returnvalue (Ability|GetAbilitySystemComponent _as_bp_katana_character_base))
  ;[1 1 1] 23-05-14 성수가 로직 수정
  (bind _returnvalue_2 (Ability|GameplayEffect|AssignTagSetbyCallerMagnitude (GameplayEffects|MakeOutgoingSpec _returnvalue "/Game/SungSoo_Workspace/Blueprints/Effects/GE_Apply_Damage.GE_Apply_Damage_C" 0.0 (GameplayEffects|MakeEffectContext _returnvalue)) "(TagName=\"Data.DamageMult\")" (Variables|Default|GetAddDamageValue)))
  (bind _returnvalue_3 (Ability|GameplayEffect|AssignTagSetbyCallerMagnitude _returnvalue_2 "(TagName=\"Data.FinalDamageRate\")" (Variables|Default|GetFinal%20Damage%20Rate)))
  (GameplayEffects|ApplyGameplayEffectSpecToTarget _returnvalue _returnvalue_3 (Ability|GetAbilitySystemComponent TargetActor)))

(event Custom|TickDamage
  (bind _boxvector (Variables|Default|GetBoxVector))
  (if (> (Variables|공격횟수|GetCrrentValue) 0)
    (Math|Integer|DecrementInt (Variables|공격횟수|GetCrrentValue)
      (:%20%20
        (Utilities|FlowControl|Sequence
          (:then_0
            (Utilities|FlowControl|DoOnce false
              (:Completed
                (CallFunction|SetBoxLocation))))
          (:then_1
            (bind (_outhits _returnvalue) (Class|KismetSystemLibrary|BoxTraceMultiforObjects _boxvector _boxvector (Variables|Default|GetHalf%20Size) (Pawn|GetControlRotation (Variables|Default|GetAs%20BP%20Katana%20Character%20Base) :!class /Script/Engine.Pawn) (Utilities|Array|MakeArray "ObjectTypeQuery3") false (Utilities|Array|MakeArray (Variables|Default|GetAs%20BP%20Katana%20Character%20Base)) "None" true))
            (if _returnvalue
              (for _array_element _outhits
                (Utilities|FlowControl|Sequence
                  (:then_0
                    (CallFunction|ApplyDamagetoTarget (.HitActor (Collision|BreakHitResult _array_element))))
                  (:then_1
                    ;[1 1 1] 히트 이펙트 스폰
                    (Class|GameplayHelperLibrary|SpawnHitEffects (Variables|Default|GetAs%20BP%20Katana%20Character%20Base) (.HitActor (Collision|BreakHitResult _array_element)) (Variables|SFX,VFX|GetAttack%20Hit%20Sound) (Variables|SFX,VFX|GetHit%20Vfx) "1.000000,1.000000,1.000000") ; HitResult는 트레이스 결과 값
                    (Camera|PlayWorldCameraShake (Variables|Default|GetShake) (Transformation|GetActorLocation) 0.0 3e+03))))))
          (:then_2
            (Utilities|FlowControl|Delay (/ (Variables|공격횟수|GetForSecond) (Math|Conversions|ToFloat(Integer) (Variables|공격횟수|GetNumExecutions))))
            (CallFunction|TickDamage)))))
    (else
      (Actor|DestroyActor))))

(event EventBeginPlay
  (bind _asbp_katana_character_base (Utilities|Casting|CastToBP_KatanaCharacterBase (Game|Player|GetPlayerPawn 0)))
  (Variables|Default|SetAs%20BP%20Katana%20Character%20Base _asbp_katana_character_base)
  (Audio|PlaySoundatLocation (Variables|SFX,VFX|GetSpawnAttackSound) (Transformation|GetActorLocation) "0, 0, 0" 1.0 1.0 0.0 0 0 0 0)
  (Variables|공격횟수|SetCrrentValue (Variables|공격횟수|GetNumExecutions))
  ;[1 1 1] 230513 성수가 로직 수정 (타이머 X 방식)
  (CallFunction|TickDamage)
  (Utilities|FlowControl|Delay (Variables|Default|GetDelayDestroyActor))
  (Actor|DestroyActor))

(event EventTick
  (params (DeltaSeconds :type Float%20%28single-precision%29))
  (CallFunction|SetBoxLocation))

(fn ConstructionScript)

(fn SetBoxLocation
  (bind _as_bp_katana_character_base (Variables|Default|GetAs%20BP%20Katana%20Character%20Base))
  (bind _as_bp_katana_character_base_2 (Variables|Default|GetAs%20BP%20Katana%20Character%20Base))
  (Transformation|SetActorLocationAndRotation (Transformation|GetActorLocation _as_bp_katana_character_base_2) (Pawn|GetControlRotation _as_bp_katana_character_base_2 :!class /Script/Engine.Pawn))
  (Variables|Default|SetBoxVector (+ (Transformation|GetActorLocation _as_bp_katana_character_base) (Math|Vector|RotateVector (Variables|Default|GetAttackBoundingBoxRelativePosition) (Pawn|GetControlRotation _as_bp_katana_character_base :!class /Script/Engine.Pawn)))))