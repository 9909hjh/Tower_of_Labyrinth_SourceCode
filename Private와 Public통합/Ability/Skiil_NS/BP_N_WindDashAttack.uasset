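; BP_N_WindDashAttack is an anim notify that performs hit detection for the katana character's wind dash attack.
; It runs a box trace for pawns at an offset from the character, oriented by either control rotation or actor rotation plus a relative rotation.
; Each hit sends an Event.Player.Ability.Hit gameplay event back to the attacker, carrying the hit result as target data and the damage multiplier as magnitude.
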(fn ReceivedNotify
  (params (MeshComp :type Skeletal%20Mesh%20Component%20Object%20Reference) (Animation :type Anim%20Sequence%20Base%20Object%20Reference) (EventReference :type Anim%20Notify%20Event%20Reference%20Structure%20%28by%20ref%29))
  (|CallParentFunction MeshComp Animation "")
  (bind _output_get (LocalVariables|SetOwner (Components|GetOwner MeshComp)))
  (bind _asbp_katana_character_base (Utilities|Casting|CastToBP_KatanaCharacterBase _output_get))
  (LocalVariables|SetKatanaBase _asbp_katana_character_base)
  (if (Variables|Default|GetbUseControllerRotation)
    (LocalVariables|SetAttackRelativeRotation "0, 0, 0")
    (LocalVariables|SetBoxLocation (+ (Transformation|GetActorLocation (LocalVariables|GetKatanaBase)) (Math|Vector|RotateVector (Variables|Default|GetAttackBoundingBoxRelativePosition) (Pawn|GetControlRotation (LocalVariables|GetKatanaBase) :!class /Script/Engine.Pawn))))
    (LocalVariables|SetBoxRotation (Pawn|GetControlRotation (LocalVariables|GetKatanaBase) :!class /Script/Engine.Pawn))
    (else
      (LocalVariables|SetAttackRelativeRotation (Variables|Default|GetAttackBoundingBoxRelativeRotation))
      (LocalVariables|SetBoxLocation (+ (Transformation|GetActorLocation (LocalVariables|GetKatanaBase)) (Math|Vector|RotateVector (Variables|Default|GetAttackBoundingBoxRelativePosition) (Transformation|GetActorRotation (LocalVariables|GetKatanaBase)))))
      (LocalVariables|SetBoxRotation (Math|Rotator|CombineRotators (Transformation|GetActorRotation (LocalVariables|GetKatanaBase)) (LocalVariables|GetAttackRelativeRotation)))))
  (bind (_outhits _returnvalue) (Class|KismetSystemLibrary|BoxTraceMultiforObjects (LocalVariables|GetBoxLocation) (LocalVariables|GetBoxLocation) (Variables|Default|GetAttackBoundingBoxExtents) (LocalVariables|GetBoxRotation) (Utilities|Array|MakeArray "ObjectTypeQuery3") false (Utilities|Array|MakeArray (LocalVariables|GetOwner)) "None" true))
  (if _returnvalue
    (for _array_element _outhits
      (Ability|SendGameplayEventtoActor (LocalVariables|GetOwner) "(TagName=\"Event.Player.Ability.Hit\")" (Utilities|Struct|MakeGameplayEventData "(TagName=\"\")" (LocalVariables|GetOwner) 0 0 0 (GameplayEffects|MakeEffectContext (Ability|GetAbilitySystemComponent (LocalVariables|GetOwner))) "(GameplayTags=)" "(GameplayTags=)" (Variables|Default|Get피해배율) (Ability|TargetData|AbilityTargetDatafromHitResult _array_element))))
    (return true)))